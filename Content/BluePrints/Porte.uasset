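; Door Blueprint that swings open or closed each time an actor overlaps it, unless it is already turning.
; An overlap flips the open state, posts the matching Wwise opening or closing sound, and starts the turn.
; Tick then steps the yaw by the turn speed, clamps it between zero and the max angle to stop, and applies it to the door mesh.
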(event `self.ReceiveBeginPlay`)

(event `self.ReceiveActorBeginOverlap`
  (params (OtherActor :type "Actor Object Reference"))
  (if (not (`self.IsTurning`))
    (bind _output_get (set `self.IsOpen` (not (`self.IsOpen`))))
    (`AkGameplayStatics.PostEvent` (select `bool` _output_get :`false` (`self.SonFermeture`) :`true` (`self.SonOuverture`)) self)
    (set `self.IsTurning` true)))

(event `self.ReceiveTick`
  (params (DeltaSeconds :type "Float (single-precision)"))
  (if (`self.IsTurning`)
    (`self.UpdateAngle` DeltaSeconds)
    (`self.Turn`)))

(fn `Turn`
  (`SceneComponent.K2_SetRelativeRotation` (`self.FBXporteV2`) (`KismetMathLibrary.MakeRotator` 0.0 0.0 (`self.Angle`)) false false))

(fn `UpdateAngle`
  (params (Delta :type "Float (double-precision)"))
  (locals (Del :type "Float (double-precision)"))
  (set `local.Del` (* Delta (`self.SpeedTurn`)))
  (if (`self.IsOpen`)
    (bind _output_get (set `self.Angle` (+ (`self.Angle`) (`local.Del`))))
    (if (>= _output_get (`self.MaxAngle`))
      (set `self.Angle` (`self.MaxAngle`))
      (set `self.IsTurning` false :!label _label))
    (else
      (bind _output_get_2 (set `self.Angle` (- (`self.Angle`) (`local.Del`))))
      (if (<= _output_get_2 0.0)
        (set `self.Angle` 0.0)
        (goto _label)))))

(fn `UserConstructionScript`
  (set `self.MaxAngle` 90.0)
  (set `self.IsTurning` false)
  (set `self.IsOpen` false)
  (set `self.Angle` 0.0))