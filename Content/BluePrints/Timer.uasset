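; Timer actor that counts elapsed time while its Defile flag is set.
; Tick adds delta seconds to the Temps accumulator whenever Defile is true.
; A Get2Digits helper converts a number to text with a leading zero below ten, though nothing in this file calls it.
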(event `self.ReceiveTick`
  (params (DeltaSeconds :type "Float (single-precision)"))
  (if (`self.Defile`)
    (set `self.Temps` (+ DeltaSeconds (`self.Temps`)))))

(fn `Get2Digits`
  (params (Num :type Integer))
  (returns (Numbers :type String))
  (return (`KismetStringLibrary.Concat_StrStr` (select `bool` (< Num 10) :`true` "0") (`KismetStringLibrary.Conv_IntToString` Num))))

(fn `UserConstructionScript`)